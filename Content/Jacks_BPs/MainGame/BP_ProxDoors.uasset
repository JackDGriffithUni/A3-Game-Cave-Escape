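; BP_ProxDoors is a proximity door that raises once when the player pawn begins overlapping it.
; BeginPlay derives the raised end position from the actor's world location and RaisedDoorHeight.
; A timeline lerps the Cube's relative location between those world-space positions while dust particles play, deactivating them on finish.
; DoorRaising blocks retriggering and is never reset, so the door does not lower.
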(event `self.ReceiveBeginPlay`
  (bind _output_get (set `self.StartingPosition` (`self.K2_GetActorLocation`)))
  (set `self.EndPosition` (`KismetMathLibrary.MakeVector` (.x _output_get) (.y _output_get) (+ (.z _output_get) (`self.RaisedDoorHeight`)))))

(event `self.ReceiveActorBeginOverlap`
  (params (OtherActor :type "Actor Object Reference"))
  (if (== OtherActor (`GameplayStatics.GetPlayerPawn` 0))
    (if (not (`self.DoorRaising`))
      (`KismetSystemLibrary.PrintString` "Door raising")
      (set `self.DoorRaising` true)
      (`ActorComponent.Activate` (`self.DustParticles`) false)
      (bind (_direction _door_raise) (`Timeline|Timeline`)
        (:`Update`
          (`SceneComponent.K2_SetRelativeLocation` (`self.Cube`) (`KismetMathLibrary.VLerp` (`self.StartingPosition`) (`self.EndPosition`) _door_raise) false true))
        (:`Finished`
          (`ActorComponent.Deactivate` (`self.DustParticles`)))))))

(fn `UserConstructionScript`)