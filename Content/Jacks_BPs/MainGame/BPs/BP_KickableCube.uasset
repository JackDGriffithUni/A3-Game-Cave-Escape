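; Physics cube that can be kicked and expires after a limited, slightly randomised lifespan.
; A looping one-second timer counts down its life, fading a dynamic material from its base colour to black.
; On expiry it destroys itself after its death sound finishes, or immediately and silently on the main menu level.
; An interface kick event applies a mass-independent impulse with upward lift and randomised spin.
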(event `self.ReceiveBeginPlay`
  (bind _maxcubelifespan (`self.MaxCubeLifespan`))
  ;[1 1 1] On spawn, set cube max lifetime, set up a dynamic material so the cube will fade to black, and run a timer that slowly depletes its lifetime
  ;;[1 1 1] Don't play cube death SFX while on the main menu
  (bind _returnvalue (`GameplayStatics.GetCurrentLevelName` true))
  (if (`KismetStringLibrary.EqualEqual_StrStr` _returnvalue "MainMenu")
    (set `self.IsMainGame` false))
  (set `self.TimeUntilDespawn` (`KismetMathLibrary.RandomFloatInRange` (* _maxcubelifespan 0.9) (* _maxcubelifespan 1.1)))
  (bind _returnvalue_2 (`PrimitiveComponent.CreateDynamicMaterialInstance` (`self.Cube`) 0 "/Game/Jacks_BPs/MainGame/Materials/M_KickableCubeMaterial.M_KickableCubeMaterial" "None"))
  (bind _returnvalue_3 (`KismetSystemLibrary.K2_SetTimerDelegate` (delegate `DeathClockTick`) 1.0 true)))

(event `DeathClockTick`
  (bind _timeuntildespawn (`self.TimeUntilDespawn`))
  (bind _cubedeathsfx (`self.CubeDeathSFX`))
  (bind (_returnvalue_r _returnvalue_g _returnvalue_b) (break `LinearColor` (`KismetMathLibrary.LinearColorLerp` (struct :`A` 0.996) (`self.BaseButtonColour`) (/ (`self.TimeUntilDespawn`) (`self.MaxCubeLifespan`)))))
  (`/Engine/EditorBlueprintResources/StandardMacros.DecrementFloat` _timeuntildespawn
    (:`  `
      (if (<= _timeuntildespawn 0.0)
        (if (`self.IsMainGame`)
          ;[1 1 1] Play cube death SFX and then destroy the cube once the SFX has finished playing
          (`KismetSystemLibrary.K2_PauseTimerHandle` (stale `self.ReceiveBeginPlay` _returnvalue_3))
          (if (not (`AudioComponent.IsPlaying` _cubedeathsfx))
            (`AudioComponent.Play` _cubedeathsfx 0.0)
            (`KismetSystemLibrary.Delay` (`SoundBase.Duration` (`AudioComponent.Sound` _cubedeathsfx)))
            (`self.K2_DestroyActor`) ; Destroy cube once lifetime expires and SFX finishes
          )
          (else
            (`self.K2_DestroyActor`) ; Destroy cube instantly when lifetime expires on the main menu
          ))
        (else
          ;[1 1 1] Slowly fade the cube from blue to black
          (`MaterialInstanceDynamic.SetVectorParameterValue` (stale `self.ReceiveBeginPlay` _returnvalue_2) "KickableCubeColour" (make `LinearColor` _returnvalue_r _returnvalue_g _returnvalue_b)))))))

(event `/Game/Jacks_BPs/MainGame/BPs/OnKicked.OnObjectKicked`
  (params (KickDirection :type "Vector Structure"))
  ;[1 1 1] Interface picks up when cube has been kicked
  (`self.KickCube` KickDirection))

(fn `KickCube`
  (params (KickDirection :type "Vector Structure"))
  (bind _kickforce (`self.KickForce`))
  (bind _returnvalue (* 2.5 _kickforce))
  (bind _returnvalue_2 (* KickDirection_X _kickforce))
  (bind _returnvalue_3 (* KickDirection_Y _kickforce))
  ;[1 1 1] Apply force and rotation on kick
  (`PrimitiveComponent.AddImpulse` (`self.Cube`) (`KismetMathLibrary.MakeVector` _returnvalue_2 _returnvalue_3 _returnvalue) "None" true)
  ;[1 1 1] Randomise the kick force for the rotation to give it some spice
  (bind _output_get (set `self.RandomRotationForce` (`KismetMathLibrary.MakeVector` (`KismetMathLibrary.RandomFloatInRange` (* _returnvalue_2 0.0) (* _returnvalue_2 1.0)) (`KismetMathLibrary.RandomFloatInRange` (* _returnvalue_3 0.0) (* _returnvalue_3 1.0)) (`KismetMathLibrary.RandomFloatInRange` (* _returnvalue -0.25) (* _returnvalue 0.25)))))
  (`PrimitiveComponent.AddAngularImpulseInDegrees` (`self.Cube`) _output_get "None" true))

(fn `UserConstructionScript`)