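; Cave escape game mode that picks a random colour code and reveals it once the cube quota is reached.
; BeginPlay builds the code by randomly removing keys from the AvailableColours map down to CodeLength, keeping their original order, and prints it to screen.
; CubeQuotaReached finds the BP_CubeCollector and starts a looping timer that cycles through the code, sending each colour's name, value and position to its display.
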(event `self.ReceiveBeginPlay`
  (bind _colourcode (`self.ColourCode`))
  (bind _keys (`BlueprintMapLibrary.Map_Keys` (`self.AvailableColours`)))
  (bind _output_get (set `self.ColourCode` _keys))
  (while (> (`KismetArrayLibrary.Array_Length` _output_get) (`self.CodeLength`))
    (`KismetArrayLibrary.Array_Remove` (`self.ColourCode`) (`KismetMathLibrary.RandomIntegerInRange` 0 (`KismetArrayLibrary.Array_Length` _colourcode))))
  (for (_array_element _array_index) _colourcode
    (`KismetSystemLibrary.PrintString` (`KismetStringLibrary.Concat_StrStr` "Colour " (`KismetStringLibrary.Conv_IntToString` (+ _array_index 1)) " = " _array_element) true true (struct :`G` 0.66 :`B` 1.0 :`A` 1.0) 5.0)))

(event `CubeQuotaReached`
  (bind _returnvalue (`GameplayStatics.GetActorOfClass` "/Game/Jacks_BPs/MainGame/BPs/BP_CubeCollector.BP_CubeCollector_C"))
  (set `self.CubeCollector` _returnvalue)
  (`KismetSystemLibrary.K2_SetTimer` null "DisplayColourCode" 2.5 true false 3.0 1.0))

(fn `DisplayColourCode`
  (bind _codedisplayindex (`self.CodeDisplayIndex`))
  (bind _output (`|GetArrayItem` (`self.ColourCode`) _codedisplayindex))
  (if (> (`self.CodeDisplayIndex`) (- (`self.CodeLength`) 1))
    (set `self.CodeDisplayIndex` 0))
  (`/Game/Jacks_BPs/MainGame/BPs/BP_CubeCollector.UpdateCodeDisplay` (`self.CubeCollector`) _output (`BlueprintMapLibrary.Map_Find` (`self.AvailableColours`) _output) (+ _codedisplayindex 1))
  (`/Engine/EditorBlueprintResources/StandardMacros.IncrementInt` (`self.CodeDisplayIndex`)))

(fn `UserConstructionScript`)