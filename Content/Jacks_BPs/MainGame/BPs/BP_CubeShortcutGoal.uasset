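; BP_CubeShortcutGoal is a goal that rewards the player when a BP_PureCube overlaps it.
; Scoring restores a percentage of the cube's lifespan, clamped to its maximum, and plays goal sound and confetti.
; It then passes an oxygen restore amount to the first-person character through OnShortcutScored.
; A short cooldown flag, cleared after a delay, prevents repeated triggers.
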(event `self.ReceiveActorBeginOverlap`
  (params (OtherActor :type "Actor Object Reference"))
  (if (`self.GoalOnCooldown`)
    _
    (elif (== (`GameplayStatics.GetObjectClass` OtherActor) "/Game/Jacks_BPs/MainGame/BPs/KickableCubes/BP_PureCube.BP_PureCube_C")
      (set `self.GoalOnCooldown` true)
      (bind _asbp_pure_cube (cast `/Game/Jacks_BPs/MainGame/BPs/KickableCubes/BP_PureCube` OtherActor))
      (bind _maxcubelifespan (`/Game/Jacks_BPs/MainGame/BPs/KickableCubes/BP_PureCube.MaxCubeLifespan` _asbp_pure_cube))
      ;[1 1 1] Restore a % of the cube's total lifespan when going through a goal (cannot restore more than max lifetime)
      (set `/Game/Jacks_BPs/MainGame/BPs/KickableCubes/BP_PureCube.TimeUntilDespawn` (`KismetMathLibrary.FClamp` (+ (`/Game/Jacks_BPs/MainGame/BPs/KickableCubes/BP_PureCube.TimeUntilDespawn` _asbp_pure_cube) (* (`self.CubeBonusLifePercent`) _maxcubelifespan)) 0.0 _maxcubelifespan) _asbp_pure_cube)
      ;[1 1 1] Play goal SFX and particles
      (`AudioComponent.Play` (`self.GoalSFX`) 0.0)
      (`ActorComponent.Activate` (`self.ConfettiParticles`) true)
      ;[1 1 1] Restore player's oxygen if goal allows for it, also play special effects when scoring
      (bind _asbp_first_person_character (cast `/Game/FirstPerson/Blueprints/BP_FirstPersonCharacter` (`GameplayStatics.GetPlayerPawn` 0)))
      (`/Game/FirstPerson/Blueprints/BP_FirstPersonCharacter.OnShortcutScored` _asbp_first_person_character (`self.RestoreOxygenAmount`))
      ;[1 1 1] Prevent "spam goals"
      (`KismetSystemLibrary.RetriggerableDelay` 0.2)
      (set `self.GoalOnCooldown` false))))

(fn `UserConstructionScript`)