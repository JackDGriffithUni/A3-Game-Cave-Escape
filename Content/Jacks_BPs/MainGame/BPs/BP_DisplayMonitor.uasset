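; BP_DisplayMonitor is an in-game monitor that shows puzzle progress on a TextRender component: cubes needed, colour code entries and exit door status.
; It exposes three display functions and contains no logic that calls them.
; The cube display switches to a code-generation message when none remain.
; Code entries show index and colour name tinted in that colour, while the exit unlocked message resets the text to the white colour variable.
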(fn `ExitUnlockedTextDisplay`
  (locals (WhiteColour :type "Color Structure" :default (struct :`B` 255 :`G` 255 :`R` 255 :`A` 255)))
  (bind _textrender (`self.TextRender`))
  (`TextRenderComponent.SetTextRenderColor` _textrender (`local.WhiteColour`))
  (`TextRenderComponent.K2_SetText` _textrender (`self.ExitDoorUnlockedText`)))

(fn `UpdateCodeDisplay`
  (params (ColourName :type String) (Colour :type "LinearColor Structure") (CodeIndex :type Integer))
  (bind _textrender (`self.TextRender`))
  (`TextRenderComponent.SetTextRenderColor` _textrender (`KismetMathLibrary.Conv_LinearColorToColor` Colour))
  (`TextRenderComponent.K2_SetText` _textrender (`KismetTextLibrary.Conv_StringToText` (`KismetStringLibrary.Concat_StrStr` "#" (`KismetStringLibrary.Conv_IntToString` CodeIndex) ": " ColourName))))

(fn `UpdateCubesLeftDisplay`
  (params (CubesRemaining :type Integer))
  (bind _textrender (`self.TextRender`))
  ;[1 1 1] Updates monitor text showing how many cubes are left, or states that a code is being generated if <= 0
  (if (> CubesRemaining 0)
    (`TextRenderComponent.K2_SetText` _textrender (`KismetTextLibrary.Conv_StringToText` (`KismetStringLibrary.Concat_StrStr` "CUBES NEEDED: " (`KismetStringLibrary.Conv_IntToString` CubesRemaining))))
    (else
      (`TextRenderComponent.K2_SetText` _textrender (`self.AllCubesText`)))))

(fn `UserConstructionScript`)