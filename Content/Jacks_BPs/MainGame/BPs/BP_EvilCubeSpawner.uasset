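; BP_EvilCubeSpawner spawns the red evil cube enemies and keeps replacing them during play.
; On BeginPlay it waits an initial delay, then spawns up to a configurable maximum at a timed interval, each at a random spawn point with a sound.
; Each cube receives a reference to the spawner, whose victory and death events schedule a replacement after a random delay, longer for deaths.
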(event `self.ReceiveBeginPlay`
  ;[1 1 1] Easy to scale up how many red cubes spawn, and how quickly they spawn after the first cube spawns
  (`KismetSystemLibrary.Delay` (`self.FirstEvilCubeSpawnDelay`))
  (for _ (range (+ (`self.MaxEvilCubes`) 1))
    (`self.SpawnEvilCube`)
    (`KismetSystemLibrary.Delay` (`self.SpawnWaveDelay`))))

(event `/Game/Jacks_BPs/MainGame/BPs/BPI_EvilCubeOutcomeReached.OnEvilCubeVictory`
  (`GameplayStatics.PlaySound2D` "/Game/Jacks_BPs/Global/Audio/SFX/EvilCubeGoalReached.EvilCubeGoalReached" 1.0 1.0 0.0 null null false)
  (`KismetSystemLibrary.Delay` (`KismetMathLibrary.RandomFloatInRange` 10.0 20.0))
  (`self.SpawnEvilCube`))

(event `/Game/Jacks_BPs/MainGame/BPs/BPI_EvilCubeOutcomeReached.OnEvilCubeDeath`
  (`KismetSystemLibrary.Delay` (`KismetMathLibrary.RandomFloatInRange` 30.0 60.0))
  (`self.SpawnEvilCube`))

(fn `SpawnEvilCube`
  (locals (SpawnPoint :type "Vector Structure"))
  (bind _output_get (set `local.SpawnPoint` (`KismetArrayLibrary.Array_Random` (`self.SpawnPoints`))))
  (bind _returnvalue (`|SpawnActorFromClass` "/Game/Jacks_BPs/MainGame/BPs/KickableCubes/BP_EvilCube.BP_EvilCube_C" (`KismetMathLibrary.Conv_VectorToTransform` _output_get) "AdjustIfPossibleButDontSpawnIfColliding" "MultiplyWithRoot" null null))
  (set `/Game/Jacks_BPs/MainGame/BPs/KickableCubes/BP_EvilCube.Spawner` self _returnvalue)
  (`GameplayStatics.PlaySound2D` "/Game/Jacks_BPs/Global/Audio/SFX/EvilCubeSpawn.EvilCubeSpawn" 1.0 1.0 0.0 null null false))

(fn `UserConstructionScript`)