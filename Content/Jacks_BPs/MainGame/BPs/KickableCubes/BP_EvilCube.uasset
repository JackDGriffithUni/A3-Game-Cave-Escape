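; BP_EvilCube is a kickable physics cube that hops along a navmesh path toward a target with randomized Y, and notifies its spawner when it falls into a pit.
; GeneratePath jitters intermediate path points for less optimal-looking movement.
; A looping timer waits until the cube is nearly still, then launches an impulse hop toward the next node, weaker at close range.
; It repaths after being kicked or taking too many hops toward one node.
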(event `self.ReceiveBeginPlay`
  (`self.GeneratePath`)
  (`KismetSystemLibrary.K2_SetTimer` null "DirectionToNextNode" 1.0 true))

(event `/Game/Jacks_BPs/MainGame/BPs/BPI_OnDeathPitContact.FellIntoPit`
  (message `/Game/Jacks_BPs/MainGame/BPs/BPI_EvilCubeOutcomeReached.OnEvilCubeDeath` (`self.Spawner`))
  (`self.K2_DestroyActor`))

(event `/Game/Jacks_BPs/MainGame/BPs/BPI_OnKicked.OnObjectKicked`
  (params (KickDirection :type "Vector Structure") (IsAirborne :type Boolean))
  ;[1 1 1] Regen path when kicked
  (set `self.RegeneratePath` true)
  (`self.KickCube` KickDirection))

(fn `DirectionToNextNode`
  (if (<= (`KismetMathLibrary.VSize` (`SceneComponent.GetComponentVelocity` (`self.Cube`))) 5.0)
    (if (`self.RegeneratePath`)
      (set `self.RegeneratePath` false)
      (`self.GeneratePath`))
    (set `self.IsHopping` false)
    (if (<= (`KismetMathLibrary.Vector_Distance` (`|GetArrayItem` (`NavigationPath.PathPoints` (`self.PathData`)) (`self.CurrentNode`)) (`self.K2_GetActorLocation`)) 100.0)
      (`/Engine/EditorBlueprintResources/StandardMacros.IncrementInt` (`self.CurrentNode`)
        (:`  `
          (set `self.CurrentHopsTowardsNode` 0))))
    (`self.HopTowardsPoint` (`|GetArrayItem` (`NavigationPath.PathPoints` (`self.PathData`)) (`self.CurrentNode`)))))

(fn `GeneratePath`
  (locals (RandomNodeVariance :type "Rotator Structure") (PathPoints :type "Array of Vector Structure"))
  (bind (_pathfindingtarget_x _pathfindingtarget_y _pathfindingtarget_z) (`KismetMathLibrary.BreakVector` (`self.PathfindingTarget`)))
  (set `self.CurrentNode` 0)
  (bind _returnvalue (`NavigationSystemV1.FindPathToLocationSynchronously` (`self.K2_GetActorLocation`) (`KismetMathLibrary.MakeVector` _pathfindingtarget_x (`KismetMathLibrary.RandomFloatInRange` -2600.0 -720.0) _pathfindingtarget_z) (`self.GetOwner`) null))
  (bind _output_get (set `self.PathData` _returnvalue))
  (bind _pathpoints (`NavigationPath.PathPoints` _output_get))
  ;[1 1 1] Randomise each pathfinding node to make the cube's path feel less 'min-maxed'
  (for (_array_element _array_index) _pathpoints
    (if (!= _array_index (`KismetArrayLibrary.Array_LastIndex` _pathpoints))
      (bind (_randomlocation _returnvalue_2) (`NavigationSystemV1.K2_GetRandomReachablePointInRadius` _array_element 200.0 null null))
      (if _returnvalue_2
        (`KismetArrayLibrary.Array_Set` _pathpoints _array_index _randomlocation)))))

(fn `HopTowardsPoint`
  (params (Target :type "Vector Structure"))
  (locals (DirectionToHop :type "Rotator Structure"))
  (bind _returnvalue (`self.K2_GetActorLocation`))
  (if (not (`self.IsHopping`))
    (bind _output_get (set `local.DirectionToHop` (`KismetMathLibrary.FindLookAtRotation` _returnvalue Target)))
    (bind (_returnvalue_x _returnvalue_y) (`KismetMathLibrary.BreakVector` (`KismetMathLibrary.GetForwardVector` _output_get)))
    ;[1 1 1] Hop towards next pathing node
    (`PrimitiveComponent.AddImpulse` (`self.Cube`) (* (`KismetMathLibrary.MakeVector` _returnvalue_x _returnvalue_y 1.0) (* (`self.JumpForce`) (`KismetMathLibrary.Lerp` 0.33 1.0 (`KismetMathLibrary.FClamp` (/ (`KismetMathLibrary.Vector_Distance` _returnvalue Target) 200.0))))) "None" true)
    (set `self.IsHopping` true)
    (`/Engine/EditorBlueprintResources/StandardMacros.IncrementInt` (`self.CurrentHopsTowardsNode`)
      (:`  `
        (if (>= (`self.CurrentHopsTowardsNode`) (`self.MaxHopsBeforeRepathing`))
          (`self.GeneratePath`))))))

(fn `UserConstructionScript`
  (`parent.UserConstructionScript`))