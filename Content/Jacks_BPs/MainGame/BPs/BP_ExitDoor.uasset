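; BP_ExitDoor is the cave escape level exit, which reacts once when the player pawn hits it.
; If the game state reports the exit unlocked, it saves stats and checks LevelToLoad.
; A MainMenu target triggers the game mode's win state and win music; any other level loads after a screen fade widget plays.
; The touched flag is set before the unlock check, so hitting a locked door also consumes it.
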(event `self.ReceiveHit`
  (params (MyComp :type "PrimitiveComponent Object Reference") (Other :type "Actor Object Reference") (OtherComp :type "PrimitiveComponent Object Reference") (bSelfMoved :type Boolean) (HitLocation :type "Vector Structure") (HitNormal :type "Vector Structure") (NormalImpulse :type "Vector Structure") (Hit :type "HitResult Structure (by ref)"))
  (if (== Other (`GameplayStatics.GetPlayerPawn` 0))
    (if (not (`self.DoorTouched`))
      (set `self.DoorTouched` true)
      ;[1 1 1] If exit is unlocked when touched, the player has beat the level!
      (bind _asgame_state_cave_escape (cast `/Game/Jacks_BPs/MainGame/BPs/GameState_CaveEscape` (`GameplayStatics.GetGameState`)))
      (if (`/Game/Jacks_BPs/MainGame/BPs/GameState_CaveEscape.ExitUnlocked` _asgame_state_cave_escape)
        (`/Game/Jacks_BPs/MainGame/BPs/GameState_CaveEscape.SaveStats` _asgame_state_cave_escape)
        (if (== (`self.LevelToLoad`) (`self.MainMenu`))
          ;[1 1 1] If heading to the main menu, the player has won!
          (bind _asgm_cave_escape (cast `/Game/Jacks_BPs/MainGame/BPs/GM_CaveEscape` (`GameplayStatics.GetGameMode`)))
          (`/Game/Jacks_BPs/MainGame/BPs/GM_CaveEscape.WinStateReached` _asgm_cave_escape)
          (`AudioComponent.Play` (`self.WinMusic`) 0.0)
          (else
            ;[1 1 1] When going to next level, fade out the view of the current level before transitioning
            (bind _returnvalue (`|CreateWidget` "/Game/Jacks_BPs/MainGame/UI/WBG_ScreenFade.WBG_ScreenFade_C"))
            (`UserWidget.AddToViewport` _returnvalue 0)
            (`/Game/Jacks_BPs/MainGame/UI/WBG_ScreenFade.StartFadeAnimation` _returnvalue 2.5 2.0 "NewEnumerator0")
            (`KismetSystemLibrary.Delay` 2.5)
            (`GameplayStatics.OpenLevel` (`self.LevelToLoad`))))))))

(fn `UserConstructionScript`)